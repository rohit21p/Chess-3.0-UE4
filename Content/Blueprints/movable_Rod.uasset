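; Movable attack-board rod for a multi-level chess game, letting a player relocate a small board with its pieces.
; At BeginPlay it resolves its squares from coordinate IDs and hides itself if unoccupied.
; On its owner's turn, clicking a rod holding under two pieces reveals adjacent hidden rods, found by index arithmetic.
; Clicking a revealed rod transfers pieces square by square from the active rod, takes over its color and toggles the turn through ChessGameMode.
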(event `self.ReceiveBeginPlay`
  (`self.setOnClick`)
  (`self.setContainsBoards`)
  (`self.hideRestMovableBoards`)
  (bind _outactors (`GameplayStatics.GetAllActorsOfClass` "/Game/Blueprints/ChessGameMode.ChessGameMode_C"))
  (set `self.GameMode` (`KismetArrayLibrary.Array_Get` _outactors)))

(event `hideRestMovableBoards`
  ;[1 1 1] hide the rest attack boards
  (if (== (`self.containsCharacter`) 0)
    (for _array_element (`self.containsBoards`)
      (`self.SetActorHiddenInGame` _array_element true)
      (`self.SetActorEnableCollision` _array_element false)
      (set `/Game/Blueprints/board_Piece.hidden` true _array_element))
    (`self.SetActorHiddenInGame` true)
    (`self.SetActorEnableCollision` false)))

(event `setOnClick`
  ;[1 1 1] set what to do on click
  (add `self.OnClicked` (delegate `do`)))

(event `do` :!signature `self.OnClicked`
  (params (TouchedActor :type "Actor Object Reference") (ButtonPressed :type "Key Structure" :default "AnyKey"))
  ;[1 1 1] set what to do on click
  (`self.onClick`))

(event `onClick`
  ;[1 1 1] do this on click
  (`self.checkAllowance`)
  (if (`self.allowance`)
    (bind _outactors (`GameplayStatics.GetAllActorsOfClass` "/Game/Blueprints/ChessGameMode.ChessGameMode_C"))
    (if (== (`/Game/Blueprints/ChessGameMode.chance` (`KismetArrayLibrary.Array_Get` _outactors)) (`self.belongsTo`))
      (if (`self.hidden`)
        _
        (elif (`self.active`)
          (`self.deactivating`)
          (set `self.active` false)
          (else
            (bind _outactors_2 (`GameplayStatics.GetAllActorsOfClass` "movable_Rod_C"))
            (for _array_element _outactors_2
              (`self.checkAdjacency` _array_element))
            (bind _outactors_3 (`GameplayStatics.GetAllActorsOfClass` "/Game/Blueprints/ChessGameMode.ChessGameMode_C"))
            (`KismetSystemLibrary.PrintString` "Hello")
            (`/Game/Blueprints/ChessGameMode.undoSelectOther` (`KismetArrayLibrary.Array_Get` _outactors_3))
            (`self.showAvailableRods`)
            (set `self.active` true)
            (bind _outactors_4 (`GameplayStatics.GetAllActorsOfClass` "/Game/Blueprints/ChessGameMode.ChessGameMode_C"))
            (set `/Game/Blueprints/ChessGameMode.whoisactive` (make `/Game/Blueprints/Character_Id` (`self.belongsTo`) "rod" (`self.index`)) (`KismetArrayLibrary.Array_Get` _outactors_4)))))
      (else
        (bind _outactors_5 (`GameplayStatics.GetAllActorsOfClass` "/Game/Blueprints/ChessGameMode.ChessGameMode_C"))
        (bind (_whoisactive_color _whoisactive_name) (break `/Game/Blueprints/Character_Id` (`/Game/Blueprints/ChessGameMode.whoisactive` (`KismetArrayLibrary.Array_Get` _outactors_5))))
        (if (and (`KismetStringLibrary.EqualEqual_StrStr` _whoisactive_name "rod") (`self.hidden`))
          (`self.swapRods`))))))

(event `checkAdjacency`
  (params (Rod :type "/Game/Blueprints/movable_Rod Object Reference"))
  (bind _availablerods (`self.AvailableRods`))
  (bind _index (`/Game/Blueprints/movable_Rod.index` Rod))
  (bind _index_2 (`self.index`))
  ;[1 1 1] find other rods which are adjacent
  (if (and (or (== (+ _index_2 4) _index) (== (+ _index_2 2) _index) (and (== (+ _index_2 1) _index) (== (mod _index_2 2) 0)) (== (+ _index_2 -4) _index) (== (+ _index_2 -2) _index) (and (== (+ _index_2 -1) _index) (not (== (mod _index_2 2) 0)))) (`Actor.bHidden` Rod))
    (`KismetArrayLibrary.Array_Set` _availablerods (`KismetArrayLibrary.Array_Length` _availablerods) Rod true)))

(event `showAvailableRods`
  ;[1 1 1] show adjacent rods to user
  (for _array_element (`self.AvailableRods`)
    (`self.SetActorHiddenInGame` _array_element false)
    (`PrimitiveComponent.SetMaterial` (`/Game/Blueprints/movable_Rod.Cylinder` _array_element) 0 "/Game/Assets/HiddenActive.HiddenActive")
    (`self.SetActorEnableCollision` _array_element true)
    (for _array_element_2 (`/Game/Blueprints/movable_Rod.containsBoards` _array_element)
      (`self.SetActorHiddenInGame` _array_element_2 false)
      (`PrimitiveComponent.SetMaterial` (`/Game/Blueprints/board_Piece.Piece` _array_element_2) 0 "/Game/Assets/HiddenActive.HiddenActive")
      (`self.SetActorEnableCollision` _array_element_2 true))))

(event `setContainsBoards`
  (bind _containsboards (`self.containsBoards`))
  ;[1 1 1] set containsBoards prop of rod
  (for _array_element (`self.containsPieces`)
    (bind _outactors (`GameplayStatics.GetAllActorsOfClass` "/Game/Blueprints/board_Piece.board_Piece_C"))
    (for _array_element_2 _outactors
      (bind (_id_x_axis _id_y_aixs _id_level) (break `/Game/Blueprints/Piece_Id` (`/Game/Blueprints/board_Piece.id` _array_element_2)))
      (if (and (`KismetStringLibrary.EqualEqual_StrStr` _id_x_axis (break `/Game/Blueprints/Piece_Id` _array_element)) (== _id_y_aixs (`.y_aixs_5_4E9AD4B24CBA9D68C22F87B4D3EBCB46` (break `/Game/Blueprints/Piece_Id` _array_element))) (== _id_level (`.level_9_6EB51A4E4C07ABE6DACD079305A4CC98` (break `/Game/Blueprints/Piece_Id` _array_element))))
        (`KismetArrayLibrary.Array_Set` _containsboards (`KismetArrayLibrary.Array_Length` _containsboards) _array_element_2 true)))))

(event `deactivating`
  ;[1 1 1] deactivate activaed rods
  (for _array_element (`self.AvailableRods`)
    (`self.SetActorHiddenInGame` _array_element true)
    (`PrimitiveComponent.SetMaterial` (`/Game/Blueprints/movable_Rod.Cylinder` _array_element) 0 "/Game/Assets/White_Piece.White_Piece")
    (`self.SetActorEnableCollision` _array_element false)
    (for _array_element_2 (`/Game/Blueprints/movable_Rod.containsBoards` _array_element)
      (`self.SetActorHiddenInGame` _array_element_2 true)
      (`PrimitiveComponent.SetMaterial` (`/Game/Blueprints/board_Piece.Piece` _array_element_2) 0 null)
      (`self.SetActorEnableCollision` _array_element_2 false))))

(event `swapRods`
  (bind _gamemode (`self.GameMode`))
  (bind _whoisactive_color (break `/Game/Blueprints/Character_Id` (`/Game/Blueprints/ChessGameMode.whoisactive` _gamemode)))
  (bind _outactors (`GameplayStatics.GetAllActorsOfClass` "movable_Rod_C"))
  (for _array_element _outactors
    (if (`/Game/Blueprints/movable_Rod.active` _array_element)
      (`self.transferPieces` (`/Game/Blueprints/movable_Rod.containsBoards` _array_element))))
  (`/Game/Blueprints/ChessGameMode.undoSelectOther` _gamemode)
  (`/Game/Blueprints/ChessGameMode.hideActiveRod` _gamemode)
  (`self.SetActorHiddenInGame` false)
  (set `self.hidden` false)
  (set `self.belongsTo` _whoisactive_color)
  (`self.SetActorEnableCollision` true)
  (`PrimitiveComponent.SetMaterial` (`self.Cylinder`) 0 "/Game/Assets/White_Piece.White_Piece")
  (for _array_element_2 (`self.containsBoards`)
    (`self.SetActorHiddenInGame` _array_element_2 false)
    (`/Game/Blueprints/board_Piece.setMaterial` _array_element_2)
    (`self.SetActorEnableCollision` _array_element_2 true))
  (bind _outactors_2 (`GameplayStatics.GetAllActorsOfClass` "/Game/Blueprints/ChessGameMode.ChessGameMode_C"))
  (`/Game/Blueprints/ChessGameMode.toggleChance` (`KismetArrayLibrary.Array_Get` _outactors_2)))

(event `transferPieces`
  (params (fromBoard :type "Array of /Game/Blueprints/board_Piece Object Reference"))
  (for (_array_element _array_index) fromBoard
    (bind _output_get (set `self.transfer` (`/Game/Blueprints/board_Piece.containscharacter` _array_element)))
    (set `/Game/Blueprints/board_Piece.hidden` true _array_element)
    (set `/Game/Blueprints/board_Piece.containscharacter` (make `/Game/Blueprints/Character_Id` 0 "noone") _array_element)
    (set `/Game/Blueprints/board_Piece.containsColor` 0 _array_element)
    (set `/Game/Blueprints/board_Piece.contains` false _array_element)
    (switch `string` (`.Name_5_F9593F8840905CC2B3A3B2A898E7B6CF` (break `/Game/Blueprints/Character_Id` _output_get))
      (:`Default`
        (bind _item (`KismetArrayLibrary.Array_Get` (`self.containsBoards`) _array_index))
        (set `/Game/Blueprints/board_Piece.containscharacter` (make `/Game/Blueprints/Character_Id` 0 "noone") _item)
        (set `/Game/Blueprints/board_Piece.contains` false _item)
        (set `/Game/Blueprints/board_Piece.containsColor` 0 _item)
        (set `/Game/Blueprints/board_Piece.hidden` false _item))
      (:`Knight`
        (`self.transferKnight` _array_index _array_element))
      (:`Bishop`
        (`self.transferBishop` _array_element _array_index))
      (:`King`
        (`self.transferKing` _array_element _array_index))
      (:`Pawn`
        (`self.transferPawn` _array_index _array_element))
      (:`Queen`
        (`self.transferQueen` _array_element _array_index))
      (:`Rook`
        (`self.transferRook` _array_index _array_element)))))

(event `transferPawn`
  (params (toIndex :type Integer) (fromBoard :type "/Game/Blueprints/board_Piece Object Reference"))
  (bind _pawn (`/Game/Blueprints/board_Piece.pawn` fromBoard))
  (bind _item (`KismetArrayLibrary.Array_Get` (`self.containsBoards`) toIndex))
  (bind (_id_color _id_name _id_index) (break `/Game/Blueprints/Character_Id` (`/Game/Blueprints/Pawn.id` _pawn)))
  (set `/Game/Blueprints/Pawn.firstTurn` false _pawn)
  (set `/Game/Blueprints/Pawn.currentlyOn` (`/Game/Blueprints/board_Piece.id` _item) _pawn)
  (`self.K2_SetActorLocation` _pawn (+ (`self.K2_GetActorLocation` _item) (0.0 0.0 13.0)) false false)
  (set `/Game/Blueprints/board_Piece.containscharacter` (make `/Game/Blueprints/Character_Id` _id_color _id_name _id_index) _item)
  (`/Game/Blueprints/board_Piece.setCharacter` _item)
  (set `/Game/Blueprints/board_Piece.contains` true _item)
  (set `/Game/Blueprints/board_Piece.containsColor` _id_color _item)
  (set `/Game/Blueprints/board_Piece.hidden` false _item))

(event `transferKing`
  (params (fromBoard :type "/Game/Blueprints/board_Piece Object Reference") (toIndex :type Integer))
  (bind _king (`/Game/Blueprints/board_Piece.king` fromBoard))
  (bind _item (`KismetArrayLibrary.Array_Get` (`self.containsBoards`) toIndex))
  (bind (_id_color _id_name _id_index) (break `/Game/Blueprints/Character_Id` (`/Game/Blueprints/King.id` _king)))
  (set `/Game/Blueprints/King.currentlyOn` (`/Game/Blueprints/board_Piece.id` _item) _king)
  (`self.K2_SetActorLocation` _king (+ (`self.K2_GetActorLocation` _item) (0.0 0.0 13.0)) false false)
  (set `/Game/Blueprints/board_Piece.containscharacter` (make `/Game/Blueprints/Character_Id` _id_color _id_name _id_index) _item)
  (`/Game/Blueprints/board_Piece.setCharacter` _item)
  (set `/Game/Blueprints/board_Piece.contains` true _item)
  (set `/Game/Blueprints/board_Piece.containsColor` _id_color _item)
  (set `/Game/Blueprints/board_Piece.hidden` false _item))

(event `transferRook`
  (params (toIndex :type Integer) (fromBoard :type "/Game/Blueprints/board_Piece Object Reference"))
  (bind _rook (`/Game/Blueprints/board_Piece.rook` fromBoard))
  (bind _item (`KismetArrayLibrary.Array_Get` (`self.containsBoards`) toIndex))
  (bind (_id_color _id_name _id_index) (break `/Game/Blueprints/Character_Id` (`/Game/Blueprints/Rook.id` _rook)))
  (set `/Game/Blueprints/Rook.currentlyOn` (`/Game/Blueprints/board_Piece.id` _item) _rook)
  (`self.K2_SetActorLocation` _rook (+ (`self.K2_GetActorLocation` _item) (0.0 0.0 13.0)) false false)
  (set `/Game/Blueprints/board_Piece.containscharacter` (make `/Game/Blueprints/Character_Id` _id_color _id_name _id_index) _item)
  (`/Game/Blueprints/board_Piece.setCharacter` _item)
  (set `/Game/Blueprints/board_Piece.contains` true _item)
  (set `/Game/Blueprints/board_Piece.containsColor` _id_color _item)
  (set `/Game/Blueprints/board_Piece.hidden` false _item))

(event `transferQueen`
  (params (fromBoard :type "/Game/Blueprints/board_Piece Object Reference") (toIndex :type Integer))
  (bind _queen (`/Game/Blueprints/board_Piece.queen` fromBoard))
  (bind _item (`KismetArrayLibrary.Array_Get` (`self.containsBoards`) toIndex))
  (bind (_id_color _id_name _id_index) (break `/Game/Blueprints/Character_Id` (`/Game/Blueprints/Queen.id` _queen)))
  (set `/Game/Blueprints/Queen.currentlyOn` (`/Game/Blueprints/board_Piece.id` _item) _queen)
  (`self.K2_SetActorLocation` _queen (+ (`self.K2_GetActorLocation` _item) (0.0 0.0 13.0)) false false)
  (set `/Game/Blueprints/board_Piece.containscharacter` (make `/Game/Blueprints/Character_Id` _id_color _id_name _id_index) _item)
  (`/Game/Blueprints/board_Piece.setCharacter` _item)
  (set `/Game/Blueprints/board_Piece.contains` true _item)
  (set `/Game/Blueprints/board_Piece.containsColor` _id_color _item)
  (set `/Game/Blueprints/board_Piece.hidden` false _item))

(event `transferKnight`
  (params (toIndex :type Integer) (fromBoard :type "/Game/Blueprints/board_Piece Object Reference"))
  (bind _knight (`/Game/Blueprints/board_Piece.knight` fromBoard))
  (bind _item (`KismetArrayLibrary.Array_Get` (`self.containsBoards`) toIndex))
  (bind (_id_color _id_name _id_index) (break `/Game/Blueprints/Character_Id` (`/Game/Blueprints/Knight.id` _knight)))
  (set `/Game/Blueprints/Knight.currentlyOn` (`/Game/Blueprints/board_Piece.id` _item) _knight)
  (`self.K2_SetActorLocation` _knight (+ (`self.K2_GetActorLocation` _item) (0.0 0.0 13.0)) false false)
  (set `/Game/Blueprints/board_Piece.containscharacter` (make `/Game/Blueprints/Character_Id` _id_color _id_name _id_index) _item)
  (`/Game/Blueprints/board_Piece.setCharacter` _item)
  (set `/Game/Blueprints/board_Piece.contains` true _item)
  (set `/Game/Blueprints/board_Piece.containsColor` _id_color _item)
  (set `/Game/Blueprints/board_Piece.hidden` false _item))

(event `transferBishop`
  (params (fromBoard :type "/Game/Blueprints/board_Piece Object Reference") (toIndex :type Integer))
  (bind _bishop (`/Game/Blueprints/board_Piece.bishop` fromBoard))
  (bind _item (`KismetArrayLibrary.Array_Get` (`self.containsBoards`) toIndex))
  (bind (_id_color _id_name _id_index) (break `/Game/Blueprints/Character_Id` (`/Game/Blueprints/Bishop.id` _bishop)))
  (set `/Game/Blueprints/Bishop.currentlyOn` (`/Game/Blueprints/board_Piece.id` _item) _bishop)
  (`self.K2_SetActorLocation` _bishop (+ (`self.K2_GetActorLocation` _item) (0.0 0.0 13.0)) false false)
  (set `/Game/Blueprints/board_Piece.containscharacter` (make `/Game/Blueprints/Character_Id` _id_color _id_name _id_index) _item)
  (`/Game/Blueprints/board_Piece.setCharacter` _item)
  (set `/Game/Blueprints/board_Piece.contains` true _item)
  (set `/Game/Blueprints/board_Piece.containsColor` _id_color _item)
  (set `/Game/Blueprints/board_Piece.hidden` false _item))

(event `checkAllowance`
  (for _array_element (`self.containsBoards`)
    (if (`/Game/Blueprints/board_Piece.contains` _array_element)
      (bind _output_get (set `self.counter` (+ (`self.counter`) 1)))
      (`KismetSystemLibrary.PrintString` (`KismetStringLibrary.Conv_IntToString` _output_get))))
  (if (< (`self.counter`) 2)
    (set `self.allowance` true)
    (else
      (set `self.allowance` false)))
  (set `self.counter` 0))

(fn `UserConstructionScript`)