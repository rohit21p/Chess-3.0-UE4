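; Game mode for a chess game with a multi-level board, coordinating piece selection, moves, captures and the turn toggle.
; On BeginPlay it caches every piece actor by type, plus all Board_Piece squares.
; Events switch on the piece type name to find the active piece, then deselect it or move it and clear its old square.
; Captured pieces are destroyed by matching color, name and index, and active squares get their material reset.
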(event `self.ReceiveBeginPlay`
  (bind _outactors (`GameplayStatics.GetAllActorsOfClass` "/Game/Blueprints/Knight.Knight_C"))
  (set `self.AllKnight` _outactors)
  (bind _outactors_2 (`GameplayStatics.GetAllActorsOfClass` "/Game/Blueprints/Bishop.Bishop_C"))
  (set `self.AllBishop` _outactors_2)
  (bind _outactors_3 (`GameplayStatics.GetAllActorsOfClass` "/Game/Blueprints/King.King_C"))
  (set `self.AllKing` _outactors_3)
  (bind _outactors_4 (`GameplayStatics.GetAllActorsOfClass` "/Game/Blueprints/Pawn.Pawn_C"))
  (set `self.AllPawn` _outactors_4)
  (bind _outactors_5 (`GameplayStatics.GetAllActorsOfClass` "/Game/Blueprints/Queen.Queen_C"))
  (set `self.AllQueen` _outactors_5)
  (bind _outactors_6 (`GameplayStatics.GetAllActorsOfClass` "/Game/Blueprints/Rook.Rook_C"))
  (set `self.AllRook` _outactors_6)
  (bind _outactors_7 (`GameplayStatics.GetAllActorsOfClass` "/Game/Blueprints/board_Piece.board_Piece_C"))
  (set `self.AllPieces` _outactors_7))

(event `self.ReceiveTick`
  (params (DeltaSeconds :type "Float (single-precision)")))

(event `undoSelectOther`
  (bind (_whoisactive_color _whoisactive_name) (break `/Game/Blueprints/Character_Id` (`self.whoisactive`)))
  (switch `string` _whoisactive_name
    (:`Knight`
      (for _array_element (`self.AllKnight`)
        (if (`/Game/Blueprints/Knight.active` _array_element)
          (`/Game/Blueprints/Knight.onClick` _array_element)
          (`self.deactivatePieces` :!label _label))))
    (:`Bishop`
      (for _array_element_2 (`self.AllBishop`)
        (if (`/Game/Blueprints/Bishop.active` _array_element_2)
          (`/Game/Blueprints/Bishop.onClick` _array_element_2)
          (goto _label))))
    (:`King`
      (for _array_element_3 (`self.AllKing`)
        (if (`/Game/Blueprints/King.active` _array_element_3)
          (`/Game/Blueprints/King.onClick` _array_element_3)
          (goto _label))))
    (:`Pawn`
      (for _array_element_4 (`self.AllPawn`)
        (if (`/Game/Blueprints/Pawn.active` _array_element_4)
          (`/Game/Blueprints/Pawn.onClick` _array_element_4)
          (goto _label))))
    (:`Queen`
      (for _array_element_5 (`self.AllQueen`)
        (if (`/Game/Blueprints/Queen.active` _array_element_5)
          (`/Game/Blueprints/Queen.onClick` _array_element_5)
          (goto _label))))
    (:`Rook`
      (for _array_element_6 (`self.AllRook`)
        (if (`/Game/Blueprints/Rook.active` _array_element_6)
          (`/Game/Blueprints/Rook.onClick` _array_element_6)
          (goto _label))))))

(event `moveSelected`
  (params (id :type "/Game/Blueprints/Piece_Id Structure"))
  (bind (_whoisactive_color _whoisactive_name) (break `/Game/Blueprints/Character_Id` (`self.whoisactive`)))
  (bind (_currentlyon_x_axis _currentlyon_y_aixs _currentlyon_level) (break `/Game/Blueprints/Piece_Id` (`/Game/Blueprints/Queen.currentlyOn` (`self.selectedQueen`))))
  (bind (_currentlyon_x_axis_2 _currentlyon_y_aixs_2 _currentlyon_level_2) (break `/Game/Blueprints/Piece_Id` (`/Game/Blueprints/Knight.currentlyOn` (`self.selectedKnight`))))
  (bind (_currentlyon_x_axis_3 _currentlyon_y_aixs_3 _currentlyon_level_3) (break `/Game/Blueprints/Piece_Id` (`/Game/Blueprints/Bishop.currentlyOn` (`self.selectedBishop`))))
  (bind (_currentlyon_x_axis_4 _currentlyon_y_aixs_4 _currentlyon_level_4) (break `/Game/Blueprints/Piece_Id` (`/Game/Blueprints/King.currentlyOn` (`self.selectedKing`))))
  (bind (_currentlyon_x_axis_5 _currentlyon_y_aixs_5 _currentlyon_level_5) (break `/Game/Blueprints/Piece_Id` (`/Game/Blueprints/Pawn.currentlyOn` (`self.selectedPawn`))))
  (bind (_currentlyon_x_axis_6 _currentlyon_y_aixs_6 _currentlyon_level_6) (break `/Game/Blueprints/Piece_Id` (`/Game/Blueprints/Rook.currentlyOn` (`self.selectedRook`))))
  (set `self.tempCurrOn` id)
  (switch `string` _whoisactive_name
    (:`Knight`
      (for _array_element (`self.AllKnight`)
        (set `self.selectedKnight` _array_element)
        (if (`/Game/Blueprints/Knight.active` _array_element)
          (`/Game/Blueprints/Knight.moveTo` (`self.selectedKnight`) (`self.moveTo`))
          (for _array_element_2 (`self.AllPieces`)
            (bind (_id_x_axis _id_y_aixs _id_level) (break `/Game/Blueprints/Piece_Id` (`/Game/Blueprints/board_Piece.id` _array_element_2)))
            (if (and (`KismetStringLibrary.EqualEqual_StrStr` _id_x_axis _currentlyon_x_axis_2) (== _id_y_aixs _currentlyon_y_aixs_2) (== _id_level _currentlyon_level_2))
              (set `/Game/Blueprints/board_Piece.contains` false _array_element_2)
              (set `/Game/Blueprints/board_Piece.containsColor` 0 _array_element_2)
              (set `/Game/Blueprints/board_Piece.containscharacter` (make `/Game/Blueprints/Character_Id` 0 "none") _array_element_2)))
          (set `/Game/Blueprints/Knight.currentlyOn` (`self.tempCurrOn`) (`self.selectedKnight`)))))
    (:`Bishop`
      (for _array_element_3 (`self.AllBishop`)
        (set `self.selectedBishop` _array_element_3)
        (if (`/Game/Blueprints/Bishop.active` _array_element_3)
          (`/Game/Blueprints/Bishop.moveTo` (`self.selectedBishop`) (`self.moveTo`))
          (for _array_element_4 (`self.AllPieces`)
            (bind (_id_x_axis_2 _id_y_aixs_2 _id_level_2) (break `/Game/Blueprints/Piece_Id` (`/Game/Blueprints/board_Piece.id` _array_element_4)))
            (if (and (`KismetStringLibrary.EqualEqual_StrStr` _id_x_axis_2 _currentlyon_x_axis_3) (== _id_y_aixs_2 _currentlyon_y_aixs_3) (== _id_level_2 _currentlyon_level_3))
              (set `/Game/Blueprints/board_Piece.contains` false _array_element_4)
              (set `/Game/Blueprints/board_Piece.containsColor` 0 _array_element_4)
              (set `/Game/Blueprints/board_Piece.containscharacter` (make `/Game/Blueprints/Character_Id` 0 "none") _array_element_4)))
          (set `/Game/Blueprints/Bishop.currentlyOn` (`self.tempCurrOn`) (`self.selectedBishop`)))))
    (:`King`
      (for _array_element_5 (`self.AllKing`)
        (set `self.selectedKing` _array_element_5)
        (if (`/Game/Blueprints/King.active` _array_element_5)
          (`/Game/Blueprints/King.moveTo` (`self.selectedKing`) (`self.moveTo`))
          (for _array_element_6 (`self.AllPieces`)
            (bind (_id_x_axis_3 _id_y_aixs_3 _id_level_3) (break `/Game/Blueprints/Piece_Id` (`/Game/Blueprints/board_Piece.id` _array_element_6)))
            (if (and (`KismetStringLibrary.EqualEqual_StrStr` _id_x_axis_3 _currentlyon_x_axis_4) (== _id_y_aixs_3 _currentlyon_y_aixs_4) (== _id_level_3 _currentlyon_level_4))
              (set `/Game/Blueprints/board_Piece.contains` false _array_element_6)
              (set `/Game/Blueprints/board_Piece.containsColor` 0 _array_element_6)
              (set `/Game/Blueprints/board_Piece.containscharacter` (make `/Game/Blueprints/Character_Id` 0 "none") _array_element_6)))
          (set `/Game/Blueprints/King.currentlyOn` (`self.tempCurrOn`) (`self.selectedKing`)))))
    (:`Pawn`
      (for _array_element_7 (`self.AllPawn`)
        (set `self.selectedPawn` _array_element_7)
        (if (`/Game/Blueprints/Pawn.active` _array_element_7)
          (`/Game/Blueprints/Pawn.moveTo` (`self.selectedPawn`) (`self.moveTo`))
          (for _array_element_8 (`self.AllPieces`)
            (bind (_id_x_axis_4 _id_y_aixs_4 _id_level_4) (break `/Game/Blueprints/Piece_Id` (`/Game/Blueprints/board_Piece.id` _array_element_8)))
            (if (and (`KismetStringLibrary.EqualEqual_StrStr` _id_x_axis_4 _currentlyon_x_axis_5) (== _id_y_aixs_4 _currentlyon_y_aixs_5) (== _id_level_4 _currentlyon_level_5))
              (set `/Game/Blueprints/board_Piece.contains` false _array_element_8)
              (set `/Game/Blueprints/board_Piece.containsColor` 0 _array_element_8)
              (set `/Game/Blueprints/board_Piece.containscharacter` (make `/Game/Blueprints/Character_Id` 0 "noone") _array_element_8)))
          (set `/Game/Blueprints/Pawn.currentlyOn` (`self.tempCurrOn`) (`self.selectedPawn`)))))
    (:`Queen`
      (for _array_element_9 (`self.AllQueen`)
        (set `self.selectedQueen` _array_element_9)
        (if (`/Game/Blueprints/Queen.active` _array_element_9)
          (`/Game/Blueprints/Queen.moveTo` (`self.selectedQueen`) (`self.moveTo`))
          (for _array_element_10 (`self.AllPieces`)
            (bind (_id_x_axis_5 _id_y_aixs_5 _id_level_5) (break `/Game/Blueprints/Piece_Id` (`/Game/Blueprints/board_Piece.id` _array_element_10)))
            (if (and (`KismetStringLibrary.EqualEqual_StrStr` _id_x_axis_5 _currentlyon_x_axis) (== _id_y_aixs_5 _currentlyon_y_aixs) (== _id_level_5 _currentlyon_level))
              (set `/Game/Blueprints/board_Piece.contains` false _array_element_10)
              (set `/Game/Blueprints/board_Piece.containsColor` 0 _array_element_10)
              (set `/Game/Blueprints/board_Piece.containscharacter` (make `/Game/Blueprints/Character_Id` 0 "noone") _array_element_10)))
          (set `/Game/Blueprints/Queen.currentlyOn` (`self.tempCurrOn`) (`self.selectedQueen`)))))
    (:`Rook`
      (for _array_element_11 (`self.AllRook`)
        (set `self.selectedRook` _array_element_11)
        (if (`/Game/Blueprints/Rook.active` _array_element_11)
          (`/Game/Blueprints/Rook.moveTo` (`self.selectedRook`) (`self.moveTo`))
          (for _array_element_12 (`self.AllPieces`)
            (bind (_id_x_axis_6 _id_y_aixs_6 _id_level_6) (break `/Game/Blueprints/Piece_Id` (`/Game/Blueprints/board_Piece.id` _array_element_12)))
            (if (and (`KismetStringLibrary.EqualEqual_StrStr` _id_x_axis_6 _currentlyon_x_axis_6) (== _id_y_aixs_6 _currentlyon_y_aixs_6) (== _id_level_6 _currentlyon_level_6))
              (set `/Game/Blueprints/board_Piece.contains` false _array_element_12)
              (set `/Game/Blueprints/board_Piece.containsColor` 0 _array_element_12)
              (set `/Game/Blueprints/board_Piece.containscharacter` (make `/Game/Blueprints/Character_Id` 0 "noone") _array_element_12)))
          (set `/Game/Blueprints/Rook.currentlyOn` (`self.tempCurrOn`) (`self.selectedRook`)))))))

(event `toggleChance`
  (if (== (`self.chance`) 1)
    (set `self.chance` 2)
    (else
      (set `self.chance` 1))))

(event `deactivatePieces`
  (for _array_element (`self.AllPieces`)
    (if (`/Game/Blueprints/board_Piece.active` _array_element)
      (`/Game/Blueprints/board_Piece.setMaterial` _array_element)
      (set `/Game/Blueprints/board_Piece.active` false _array_element))))

(event `deleteAlreadyCharacter`
  (params (CharacterId :type "/Game/Blueprints/Character_Id Structure"))
  (bind (_characteridtodelete_color _characteridtodelete_name _characteridtodelete_index) (break `/Game/Blueprints/Character_Id` (`self.characterIdToDelete`)))
  (bind (_characteridtodelete_color_2 _characteridtodelete_name_2 _characteridtodelete_index_2) (break `/Game/Blueprints/Character_Id` (`self.characterIdToDelete`)))
  (bind (_characteridtodelete_color_3 _characteridtodelete_name_3 _characteridtodelete_index_3) (break `/Game/Blueprints/Character_Id` (`self.characterIdToDelete`)))
  (bind (_characteridtodelete_color_4 _characteridtodelete_name_4 _characteridtodelete_index_4) (break `/Game/Blueprints/Character_Id` (`self.characterIdToDelete`)))
  (bind (_characteridtodelete_color_5 _characteridtodelete_name_5 _characteridtodelete_index_5) (break `/Game/Blueprints/Character_Id` (`self.characterIdToDelete`)))
  (bind (_characteridtodelete_color_6 _characteridtodelete_name_6 _characteridtodelete_index_6) (break `/Game/Blueprints/Character_Id` (`self.characterIdToDelete`)))
  (bind _output_get (set `self.characterIdToDelete` CharacterId))
  (switch `string` (`.Name_5_F9593F8840905CC2B3A3B2A898E7B6CF` (break `/Game/Blueprints/Character_Id` _output_get))
    (:`Knight`
      (for _array_element (`self.AllKnight`)
        (bind (_id_color _id_name _id_index) (break `/Game/Blueprints/Character_Id` (`/Game/Blueprints/Knight.id` _array_element)))
        (if (and (== _id_color _characteridtodelete_color_2) (`KismetStringLibrary.EqualEqual_StrStr` _id_name _characteridtodelete_name_2) (== _id_index _characteridtodelete_index_2))
          (`self.K2_DestroyActor` _array_element))))
    (:`Bishop`
      (for _array_element_2 (`self.AllBishop`)
        (bind (_id_color_2 _id_name_2 _id_index_2) (break `/Game/Blueprints/Character_Id` (`/Game/Blueprints/Bishop.id` _array_element_2)))
        (if (and (== _id_color_2 _characteridtodelete_color_3) (`KismetStringLibrary.EqualEqual_StrStr` _id_name_2 _characteridtodelete_name_3) (== _id_index_2 _characteridtodelete_index_3))
          (`self.K2_DestroyActor` _array_element_2))))
    (:`King`
      (for _array_element_3 (`self.AllKing`)
        (bind (_id_color_3 _id_name_3 _id_index_3) (break `/Game/Blueprints/Character_Id` (`/Game/Blueprints/King.id` _array_element_3)))
        (if (and (== _id_color_3 _characteridtodelete_color) (`KismetStringLibrary.EqualEqual_StrStr` _id_name_3 _characteridtodelete_name) (== _id_index_3 _characteridtodelete_index))
          (`self.K2_DestroyActor` _array_element_3))))
    (:`Pawn`
      (for _array_element_4 (`self.AllPawn`)
        (bind (_id_color_4 _id_name_4 _id_index_4) (break `/Game/Blueprints/Character_Id` (`/Game/Blueprints/Pawn.id` _array_element_4)))
        (if (and (== _id_color_4 _characteridtodelete_color_4) (`KismetStringLibrary.EqualEqual_StrStr` _id_name_4 _characteridtodelete_name_4) (== _id_index_4 _characteridtodelete_index_4))
          (`self.K2_DestroyActor` _array_element_4))))
    (:`Queen`
      (for _array_element_5 (`self.AllQueen`)
        (bind (_id_color_5 _id_name_5 _id_index_5) (break `/Game/Blueprints/Character_Id` (`/Game/Blueprints/Queen.id` _array_element_5)))
        (if (and (== _id_color_5 _characteridtodelete_color_6) (`KismetStringLibrary.EqualEqual_StrStr` _id_name_5 _characteridtodelete_name_6) (== _id_index_5 _characteridtodelete_index_6))
          (`self.K2_DestroyActor` _array_element_5))))
    (:`Rook`
      (for _array_element_6 (`self.AllRook`)
        (bind (_id_color_6 _id_name_6 _id_index_6) (break `/Game/Blueprints/Character_Id` (`/Game/Blueprints/Rook.id` _array_element_6)))
        (if (and (== _id_color_6 _characteridtodelete_color_5) (`KismetStringLibrary.EqualEqual_StrStr` _id_name_6 _characteridtodelete_name_5) (== _id_index_6 _characteridtodelete_index_5))
          (`self.K2_DestroyActor` _array_element_6))))))

(fn `UserConstructionScript`)