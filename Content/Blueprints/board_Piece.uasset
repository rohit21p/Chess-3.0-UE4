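; Chessboard square actor that takes a white or black material from its Color and serves as a clickable move destination.
; On BeginPlay it finds the ChessGameMode actor and binds its click event.
; When clicked while Active, it tells the game mode to move the selected piece just above it, deactivate pieces and delete any previous occupant.
; It then records the moved character's color, name and index as its occupant.
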(event `self.ReceiveBeginPlay`
  (`self.setMaterial`)
  (`self.setOnClickEvent`)
  (bind _outactors (`GameplayStatics.GetAllActorsOfClass` "/Game/Blueprints/ChessGameMode.ChessGameMode_C"))
  (for _array_element _outactors
    (set `self.gameMode` _array_element)))

(event `self.ReceiveTick`
  (params (DeltaSeconds :type "Float (single-precision)")))

(event `setMaterial`
  ;[1 1 1] set Color
  (if (== (`self.Color`) 1)
    (`PrimitiveComponent.SetMaterial` (`self.Piece`) 0 "/Game/Assets/White_Piece.White_Piece")
    (else
      (`PrimitiveComponent.SetMaterial` (`self.Piece`) 0 "/Game/Assets/Black_Piece.Black_Piece"))))

(event `setOnClickEvent`
  ;[1 1 1] Set what to do on click
  (add `self.OnClicked` (delegate `do`)))

(event `do` :!signature `self.OnClicked`
  (params (TouchedActor :type "Actor Object Reference") (ButtonPressed :type "Key Structure" :default "AnyKey"))
  ;[1 1 1] Set what to do on click
  (`self.onClick`))

(event `onClick`
  (bind (_whoisactive_color _whoisactive_name _whoisactive_index) (break `/Game/Blueprints/Character_Id` (`/Game/Blueprints/ChessGameMode.whoisactive` (`self.gameMode`))))
  (if (`self.active`)
    (set `/Game/Blueprints/ChessGameMode.moveTo` (+ (`self.K2_GetActorLocation`) (0.0 0.0 13.0)) (`self.gameMode`))
    (`/Game/Blueprints/ChessGameMode.moveSelected` (`self.gameMode`) (`self.id`))
    (`/Game/Blueprints/ChessGameMode.deactivatePieces` (`self.gameMode`))
    (`/Game/Blueprints/ChessGameMode.deleteAlreadyCharacter` (`self.gameMode`) (`self.containscharacter`))
    (set `self.containsColor` _whoisactive_color)
    (set `self.contains` true)
    (set `self.containscharacter` (make `/Game/Blueprints/Character_Id` _whoisactive_color _whoisactive_name _whoisactive_index))))

(fn `UserConstructionScript`)