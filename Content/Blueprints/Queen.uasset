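; Queen chess piece actor that handles click selection, move highlighting and relocation, coordinating turns through ChessGameMode.
; On click during its color's turn, it gathers candidate squares in eight rook and bishop directions by scanning all Board_Piece actors.
; Each direction tracks its nearest occupied square, trims squares beyond it, and merges the rest into one list to highlight and activate.
; MoveTo relocates the piece, clears the lists and toggles the turn.
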(event `self.ReceiveBeginPlay`
  (`self.setMaterial`)
  (`self.setOnClickEvent`)
  (bind _outactors (`GameplayStatics.GetAllActorsOfClass` "/Game/Blueprints/ChessGameMode.ChessGameMode_C"))
  (set `self.gameMode` (`KismetArrayLibrary.Array_Get` _outactors)))

(event `self.ReceiveTick`
  (params (DeltaSeconds :type "Float (single-precision)")))

(event `setMaterial`
  ;[1 1 1] set Color
  (if (== (`self.Color`) 1)
    (`PrimitiveComponent.SetMaterial` (`self.Queen`) 0 "/Game/Assets/White_Piece.White_Piece")
    (else
      (`PrimitiveComponent.SetMaterial` (`self.Queen`) 0 "/Game/Assets/Black_Piece.Black_Piece"))))

(event `setOnClickEvent`
  ;[1 1 1] Set what to do on click
  (add `self.OnClicked` (delegate `do`)))

(event `do` :!signature `self.OnClicked`
  (params (TouchedActor :type "Actor Object Reference") (ButtonPressed :type "Key Structure" :default "AnyKey"))
  ;[1 1 1] Set what to do on click
  (`self.onClick`))

(event `onClick`
  ;[1 1 1] on click
  (if (== (`/Game/Blueprints/ChessGameMode.chance` (`self.gameMode`)) (`self.color`))
    (if (`self.active`)
      (set `self.active` false)
      (`self.setMaterial`)
      (`/Game/Blueprints/ChessGameMode.deactivatePieces` (`self.gameMode`))
      (`self.setAllArrayToDefaults`)
      (else
        (`PrimitiveComponent.SetMaterial` (`self.Queen`) 0 "/Game/Assets/Active_Piece.Active_Piece")
        (`/Game/Blueprints/ChessGameMode.undoSelectOther` (`self.gameMode`))
        (set `self.active` true)
        (set `/Game/Blueprints/ChessGameMode.whoisactive` (`self.id`) (`self.gameMode`))
        (`self.setAvailableLocation`)
        (`self.makeAvailableLocationActive`)))))

(event `moveTo`
  (params (Location :type "Vector Structure"))
  ;[1 1 1] move Queen to new piece
  (`self.K2_SetActorLocation` Location)
  (`self.onClick`)
  (`self.setAllArrayToDefaults`)
  (`/Game/Blueprints/ChessGameMode.toggleChance` (`self.gameMode`)))

(event `setAllArrayToDefaults`
  ;[1 1 1] reset all array to defaults
  (`KismetArrayLibrary.Array_Clear` (`self.newAvailableLocation`))
  (`KismetArrayLibrary.Array_Clear` (`self.new45DLocation`))
  (`KismetArrayLibrary.Array_Clear` (`self.new135DLocation`))
  (`KismetArrayLibrary.Array_Clear` (`self.new225DLocation`))
  (`KismetArrayLibrary.Array_Clear` (`self.new315Dlocation`))
  (`KismetArrayLibrary.Array_Clear` (`self.newAvailableLocationRight`))
  (`KismetArrayLibrary.Array_Clear` (`self.newAvailableLocationLeft`))
  (`KismetArrayLibrary.Array_Clear` (`self.newAvailableLocationBack`))
  (`KismetArrayLibrary.Array_Clear` (`self.newAvailableLocationFront`)))

(event `makeAvailableLocationActive`
  ;[1 1 1] make all available location active
  (for _array_element (`self.NewAvailableLocation`)
    (bind _outactors (`GameplayStatics.GetAllActorsOfClass` "/Game/Blueprints/board_Piece.board_Piece_C"))
    (for _array_element_2 _outactors
      (bind (_id_x_axis _id_y_aixs _id_level) (break `/Game/Blueprints/Piece_Id` (`/Game/Blueprints/board_Piece.id` _array_element_2)))
      (if (and (`KismetStringLibrary.EqualEqual_StrStr` _id_x_axis (break `/Game/Blueprints/Piece_Id` _array_element)) (== _id_y_aixs (`.y_aixs_5_4E9AD4B24CBA9D68C22F87B4D3EBCB46` (break `/Game/Blueprints/Piece_Id` _array_element))) (== _id_level (`.level_9_6EB51A4E4C07ABE6DACD079305A4CC98` (break `/Game/Blueprints/Piece_Id` _array_element))))
        (`PrimitiveComponent.SetMaterial` (`/Game/Blueprints/board_Piece.Piece` _array_element_2) 0 "/Game/Assets/Active_Piece.Active_Piece")
        (set `/Game/Blueprints/board_Piece.active` true _array_element_2)))))

(event `setAvailableLocation`
  (bind _newavailablelocation (`self.newAvailableLocation`))
  (bind _newavailablelocation_2 (`self.newAvailableLocation`))
  (bind _newavailablelocation_3 (`self.newAvailableLocation`))
  (bind _newavailablelocation_4 (`self.newAvailableLocation`))
  (bind _newavailablelocation_5 (`self.newAvailableLocation`))
  (bind _newavailablelocation_6 (`self.newAvailableLocation`))
  (bind _newavailablelocation_7 (`self.newAvailableLocation`))
  (bind _newavailablelocation_8 (`self.newAvailableLocation`))
  ;[1 1 1] find all available locations
  (`self.find135Dlocations`)
  (`self.find225DLocations`)
  (`self.find315Locations`)
  (`self.find45DLocations`)
  (`self.findFrontLocation`)
  (`self.findSideLocation`)
  (`self.findRIghtLocation`)
  (`self.findBackLocation`)
  (`self.removeBlockedPieces`)
  (for _array_element (`self.new45DLocation`)
    (`KismetArrayLibrary.Array_Set` _newavailablelocation_6 (`KismetArrayLibrary.Array_Length` _newavailablelocation_6) _array_element true))
  (for _array_element_2 (`self.new135DLocation`)
    (`KismetArrayLibrary.Array_Set` _newavailablelocation_7 (`KismetArrayLibrary.Array_Length` _newavailablelocation_7) _array_element_2 true))
  (for _array_element_3 (`self.new225DLocation`)
    (`KismetArrayLibrary.Array_Set` _newavailablelocation_8 (`KismetArrayLibrary.Array_Length` _newavailablelocation_8) _array_element_3 true))
  (for _array_element_4 (`self.new315Dlocation`)
    (`KismetArrayLibrary.Array_Set` _newavailablelocation_2 (`KismetArrayLibrary.Array_Length` _newavailablelocation_2) _array_element_4 true))
  (for _array_element_5 (`self.newAvailableLocationLeft`)
    (`KismetArrayLibrary.Array_Set` _newavailablelocation_3 (`KismetArrayLibrary.Array_Length` _newavailablelocation_3) _array_element_5 true))
  (for _array_element_6 (`self.newAvailableLocationRight`)
    (`KismetArrayLibrary.Array_Set` _newavailablelocation_4 (`KismetArrayLibrary.Array_Length` _newavailablelocation_4) _array_element_6 true))
  (for _array_element_7 (`self.newAvailableLocationBack`)
    (`KismetArrayLibrary.Array_Set` _newavailablelocation_5 (`KismetArrayLibrary.Array_Length` _newavailablelocation_5) _array_element_7 true))
  (for _array_element_8 (`self.newAvailableLocationFront`)
    (`KismetArrayLibrary.Array_Set` _newavailablelocation (`KismetArrayLibrary.Array_Length` _newavailablelocation) _array_element_8 true)))

(event `find45DLocations`
  (bind (_currentlyon_x_axis _currentlyon_y_aixs) (break `/Game/Blueprints/Piece_Id` (`self.currentlyOn`)))
  (bind _new45dlocation (`self.new45DLocation`))
  (bind (_45dblockson_x_axis _45dblockson_y_aixs) (break `/Game/Blueprints/Piece_Id` (`self.45DBlocksOn`)))
  ;[1 1 1] find locations at 45deg of bishop
  (set `self.45DBlocksOn` (make `/Game/Blueprints/Piece_Id` "z" 9))
  (bind _outactors (`GameplayStatics.GetAllActorsOfClass` "/Game/Blueprints/board_Piece.board_Piece_C"))
  (for _array_element _outactors
    (bind (_id_x_axis _id_y_aixs _id_level) (break `/Game/Blueprints/Piece_Id` (`/Game/Blueprints/board_Piece.id` _array_element)))
    (bind _returnvalue (== (- (`KismetStringLibrary.GetCharacterAsNumber` _id_x_axis) (`KismetStringLibrary.GetCharacterAsNumber` _currentlyon_x_axis)) (- _id_y_aixs _currentlyon_y_aixs)))
    (bind _returnvalue_2 (> _id_y_aixs _currentlyon_y_aixs))
    (if (and _returnvalue _returnvalue_2 (!= (`/Game/Blueprints/board_Piece.containsColor` _array_element) (`self.color`)))
      (`KismetArrayLibrary.Array_Set` _new45dlocation (`KismetArrayLibrary.Array_Length` _new45dlocation) (make `/Game/Blueprints/Piece_Id` _id_x_axis _id_y_aixs _id_level) true))
    (if (and _returnvalue _returnvalue_2 (`/Game/Blueprints/board_Piece.contains` _array_element))
      (if (< _id_y_aixs _45dblockson_y_aixs)
        (set `self.45DBlocksOn` (make `/Game/Blueprints/Piece_Id` _id_x_axis _id_y_aixs _id_level)))))
  (set `self.copyOf45DLocs` (`self.new45DLocation`)))

(event `find135Dlocations`
  (bind (_currentlyon_x_axis _currentlyon_y_aixs) (break `/Game/Blueprints/Piece_Id` (`self.currentlyOn`)))
  (bind _new135dlocation (`self.new135DLocation`))
  (bind (_135dblockson_x_axis _135dblockson_y_aixs) (break `/Game/Blueprints/Piece_Id` (`self.135DBlocksOn`)))
  ;[1 1 1] find locations at 135deg of bishop
  (set `self.135DBlocksOn` (make `/Game/Blueprints/Piece_Id` "a" 9))
  (bind _outactors (`GameplayStatics.GetAllActorsOfClass` "/Game/Blueprints/board_Piece.board_Piece_C"))
  (for _array_element _outactors
    (bind (_id_x_axis _id_y_aixs _id_level) (break `/Game/Blueprints/Piece_Id` (`/Game/Blueprints/board_Piece.id` _array_element)))
    (bind _returnvalue (== (- (`KismetStringLibrary.GetCharacterAsNumber` _id_x_axis) (`KismetStringLibrary.GetCharacterAsNumber` _currentlyon_x_axis)) (* (- _id_y_aixs _currentlyon_y_aixs) -1)))
    (bind _returnvalue_2 (> _id_y_aixs _currentlyon_y_aixs))
    (if (and _returnvalue _returnvalue_2 (!= (`/Game/Blueprints/board_Piece.containsColor` _array_element) (`self.color`)))
      (`KismetArrayLibrary.Array_Set` _new135dlocation (`KismetArrayLibrary.Array_Length` _new135dlocation) (make `/Game/Blueprints/Piece_Id` _id_x_axis _id_y_aixs _id_level) true))
    (if (and _returnvalue _returnvalue_2 (`/Game/Blueprints/board_Piece.contains` _array_element))
      (if (< _id_y_aixs _135dblockson_y_aixs)
        (set `self.135DBlocksOn` (make `/Game/Blueprints/Piece_Id` _id_x_axis _id_y_aixs _id_level)))))
  (set `self.copyOf135DLocs` (`self.new135DLocation`)))

(event `find225DLocations`
  (bind (_currentlyon_x_axis _currentlyon_y_aixs) (break `/Game/Blueprints/Piece_Id` (`self.currentlyOn`)))
  (bind _new225dlocation (`self.new225DLocation`))
  (bind (_225dblockson_x_axis _225dblockson_y_aixs) (break `/Game/Blueprints/Piece_Id` (`self.225DBlocksOn`)))
  ;[1 1 1] find locations at 225deg from bishop
  (set `self.225DBlocksOn` (make `/Game/Blueprints/Piece_Id` "a"))
  (bind _outactors (`GameplayStatics.GetAllActorsOfClass` "/Game/Blueprints/board_Piece.board_Piece_C"))
  (for _array_element _outactors
    (bind (_id_x_axis _id_y_aixs _id_level) (break `/Game/Blueprints/Piece_Id` (`/Game/Blueprints/board_Piece.id` _array_element)))
    (bind _returnvalue (== (- (`KismetStringLibrary.GetCharacterAsNumber` _id_x_axis) (`KismetStringLibrary.GetCharacterAsNumber` _currentlyon_x_axis)) (- _id_y_aixs _currentlyon_y_aixs)))
    (bind _returnvalue_2 (> _currentlyon_y_aixs _id_y_aixs))
    (if (and _returnvalue _returnvalue_2 (!= (`/Game/Blueprints/board_Piece.containsColor` _array_element) (`self.color`)))
      (`KismetArrayLibrary.Array_Set` _new225dlocation (`KismetArrayLibrary.Array_Length` _new225dlocation) (make `/Game/Blueprints/Piece_Id` _id_x_axis _id_y_aixs _id_level) true))
    (if (and _returnvalue _returnvalue_2 (`/Game/Blueprints/board_Piece.contains` _array_element))
      (if (< _225dblockson_y_aixs _id_y_aixs)
        (set `self.225DBlocksOn` (make `/Game/Blueprints/Piece_Id` _id_x_axis _id_y_aixs _id_level)))))
  (set `self.copyOf225DLocs` (`self.new225DLocation`)))

(event `find315Locations`
  (bind (_currentlyon_x_axis _currentlyon_y_aixs) (break `/Game/Blueprints/Piece_Id` (`self.currentlyOn`)))
  (bind _new315dlocation (`self.new315Dlocation`))
  (bind (_315dblockson_x_axis _315dblockson_y_aixs) (break `/Game/Blueprints/Piece_Id` (`self.315DBlocksOn`)))
  ;[1 1 1] find locations at 315deg of bishop
  (set `self.315DBlocksOn` (make `/Game/Blueprints/Piece_Id` "f"))
  (bind _outactors (`GameplayStatics.GetAllActorsOfClass` "/Game/Blueprints/board_Piece.board_Piece_C"))
  (for _array_element _outactors
    (bind (_id_x_axis _id_y_aixs _id_level) (break `/Game/Blueprints/Piece_Id` (`/Game/Blueprints/board_Piece.id` _array_element)))
    (bind _returnvalue (== (- (`KismetStringLibrary.GetCharacterAsNumber` _id_x_axis) (`KismetStringLibrary.GetCharacterAsNumber` _currentlyon_x_axis)) (* (- _id_y_aixs _currentlyon_y_aixs) -1)))
    (bind _returnvalue_2 (> _currentlyon_y_aixs _id_y_aixs))
    (if (and _returnvalue _returnvalue_2 (!= (`/Game/Blueprints/board_Piece.containsColor` _array_element) (`self.color`)))
      (`KismetArrayLibrary.Array_Set` _new315dlocation (`KismetArrayLibrary.Array_Length` _new315dlocation) (make `/Game/Blueprints/Piece_Id` _id_x_axis _id_y_aixs _id_level) true))
    (if (and _returnvalue _returnvalue_2 (`/Game/Blueprints/board_Piece.contains` _array_element))
      (if (< _315dblockson_y_aixs _id_y_aixs)
        (set `self.315DBlocksOn` (make `/Game/Blueprints/Piece_Id` _id_x_axis _id_y_aixs _id_level)))))
  (set `self.copyOf315DLocs` (`self.new315Dlocation`)))

(event `removeBlockedPieces`
  (bind (_backblockon_x_axis _backblockon_y_aixs) (break `/Game/Blueprints/Piece_Id` (`self.backBlockOn`)))
  (bind (_315dblockson_x_axis _315dblockson_y_aixs) (break `/Game/Blueprints/Piece_Id` (`self.315DBlocksOn`)))
  (bind (_45dblockson_x_axis _45dblockson_y_aixs) (break `/Game/Blueprints/Piece_Id` (`self.45DBlocksOn`)))
  (bind _leftblockon_x_axis (break `/Game/Blueprints/Piece_Id` (`self.leftBlockOn`)))
  (bind (_fronblockon_x_axis _fronblockon_y_aixs) (break `/Game/Blueprints/Piece_Id` (`self.fronBlockOn`)))
  (bind (_135dblockson_x_axis _135dblockson_y_aixs) (break `/Game/Blueprints/Piece_Id` (`self.135DBlocksOn`)))
  (bind _rightblockon_x_axis (break `/Game/Blueprints/Piece_Id` (`self.rightBlockOn`)))
  (bind (_225dblockson_x_axis _225dblockson_y_aixs) (break `/Game/Blueprints/Piece_Id` (`self.225DBlocksOn`)))
  ;[1 1 1] remove invalid locations
  (for _array_element (`self.copyOf45DLocs`)
    (if (> (`.y_aixs_5_4E9AD4B24CBA9D68C22F87B4D3EBCB46` (break `/Game/Blueprints/Piece_Id` _array_element)) _45dblockson_y_aixs)
      (`KismetArrayLibrary.Array_RemoveItem` (`self.new45DLocation`) (make `/Game/Blueprints/Piece_Id` (break `/Game/Blueprints/Piece_Id` _array_element) (`.y_aixs_5_4E9AD4B24CBA9D68C22F87B4D3EBCB46` (break `/Game/Blueprints/Piece_Id` _array_element)) (`.level_9_6EB51A4E4C07ABE6DACD079305A4CC98` (break `/Game/Blueprints/Piece_Id` _array_element))))))
  (for _array_element_2 (`self.copyOf135DLocs`)
    (if (> (`.y_aixs_5_4E9AD4B24CBA9D68C22F87B4D3EBCB46` (break `/Game/Blueprints/Piece_Id` _array_element_2)) _135dblockson_y_aixs)
      (`KismetArrayLibrary.Array_RemoveItem` (`self.new135DLocation`) (make `/Game/Blueprints/Piece_Id` (break `/Game/Blueprints/Piece_Id` _array_element_2) (`.y_aixs_5_4E9AD4B24CBA9D68C22F87B4D3EBCB46` (break `/Game/Blueprints/Piece_Id` _array_element_2)) (`.level_9_6EB51A4E4C07ABE6DACD079305A4CC98` (break `/Game/Blueprints/Piece_Id` _array_element_2))))))
  (for _array_element_3 (`self.copyOf225DLocs`)
    (if (> _225dblockson_y_aixs (`.y_aixs_5_4E9AD4B24CBA9D68C22F87B4D3EBCB46` (break `/Game/Blueprints/Piece_Id` _array_element_3)))
      (`KismetArrayLibrary.Array_RemoveItem` (`self.new225DLocation`) (make `/Game/Blueprints/Piece_Id` (break `/Game/Blueprints/Piece_Id` _array_element_3) (`.y_aixs_5_4E9AD4B24CBA9D68C22F87B4D3EBCB46` (break `/Game/Blueprints/Piece_Id` _array_element_3)) (`.level_9_6EB51A4E4C07ABE6DACD079305A4CC98` (break `/Game/Blueprints/Piece_Id` _array_element_3))))))
  (for _array_element_4 (`self.copyOf315DLocs`)
    (if (> _315dblockson_y_aixs (`.y_aixs_5_4E9AD4B24CBA9D68C22F87B4D3EBCB46` (break `/Game/Blueprints/Piece_Id` _array_element_4)))
      (`KismetArrayLibrary.Array_RemoveItem` (`self.new315Dlocation`) (make `/Game/Blueprints/Piece_Id` (break `/Game/Blueprints/Piece_Id` _array_element_4) (`.y_aixs_5_4E9AD4B24CBA9D68C22F87B4D3EBCB46` (break `/Game/Blueprints/Piece_Id` _array_element_4)) (`.level_9_6EB51A4E4C07ABE6DACD079305A4CC98` (break `/Game/Blueprints/Piece_Id` _array_element_4))))))
  (for _array_element_5 (`self.copyOfLeftLocs`)
    (if (< (`KismetStringLibrary.GetCharacterAsNumber` (break `/Game/Blueprints/Piece_Id` _array_element_5)) (`KismetStringLibrary.GetCharacterAsNumber` _leftblockon_x_axis))
      (`KismetArrayLibrary.Array_RemoveItem` (`self.newAvailableLocationLeft`) (make `/Game/Blueprints/Piece_Id` (break `/Game/Blueprints/Piece_Id` _array_element_5) (`.y_aixs_5_4E9AD4B24CBA9D68C22F87B4D3EBCB46` (break `/Game/Blueprints/Piece_Id` _array_element_5)) (`.level_9_6EB51A4E4C07ABE6DACD079305A4CC98` (break `/Game/Blueprints/Piece_Id` _array_element_5))))))
  (for _array_element_6 (`self.copyOfRightLocs`)
    (if (> (`KismetStringLibrary.GetCharacterAsNumber` (break `/Game/Blueprints/Piece_Id` _array_element_6)) (`KismetStringLibrary.GetCharacterAsNumber` _rightblockon_x_axis))
      (`KismetArrayLibrary.Array_RemoveItem` (`self.newAvailableLocationRight`) (make `/Game/Blueprints/Piece_Id` (break `/Game/Blueprints/Piece_Id` _array_element_6) (`.y_aixs_5_4E9AD4B24CBA9D68C22F87B4D3EBCB46` (break `/Game/Blueprints/Piece_Id` _array_element_6)) (`.level_9_6EB51A4E4C07ABE6DACD079305A4CC98` (break `/Game/Blueprints/Piece_Id` _array_element_6))))))
  (for _array_element_7 (`self.copyOfBackLocs`)
    (if (< (`.y_aixs_5_4E9AD4B24CBA9D68C22F87B4D3EBCB46` (break `/Game/Blueprints/Piece_Id` _array_element_7)) _backblockon_y_aixs)
      (`KismetArrayLibrary.Array_RemoveItem` (`self.newAvailableLocationBack`) (make `/Game/Blueprints/Piece_Id` (break `/Game/Blueprints/Piece_Id` _array_element_7) (`.y_aixs_5_4E9AD4B24CBA9D68C22F87B4D3EBCB46` (break `/Game/Blueprints/Piece_Id` _array_element_7)) (`.level_9_6EB51A4E4C07ABE6DACD079305A4CC98` (break `/Game/Blueprints/Piece_Id` _array_element_7))))
      (`KismetSystemLibrary.PrintString` (`KismetStringLibrary.Concat_StrStr` "removed " (break `/Game/Blueprints/Piece_Id` _array_element_7) (`KismetStringLibrary.Conv_IntToString` (`.y_aixs_5_4E9AD4B24CBA9D68C22F87B4D3EBCB46` (break `/Game/Blueprints/Piece_Id` _array_element_7)))))))
  (for (_array_element_8 _array_index) (`self.copyOfFrontLocs`)
    (if (> (`.y_aixs_5_4E9AD4B24CBA9D68C22F87B4D3EBCB46` (break `/Game/Blueprints/Piece_Id` _array_element_8)) _fronblockon_y_aixs)
      (`KismetArrayLibrary.Array_RemoveItem` (`self.newAvailableLocationFront`) (make `/Game/Blueprints/Piece_Id` (break `/Game/Blueprints/Piece_Id` _array_element_8) (`.y_aixs_5_4E9AD4B24CBA9D68C22F87B4D3EBCB46` (break `/Game/Blueprints/Piece_Id` _array_element_8)) (`.level_9_6EB51A4E4C07ABE6DACD079305A4CC98` (break `/Game/Blueprints/Piece_Id` _array_element_8)))))))

(event `findFrontLocation`
  (bind (_currentlyon_x_axis _currentlyon_y_aixs) (break `/Game/Blueprints/Piece_Id` (`self.currentlyOn`)))
  (bind _newavailablelocationfront (`self.newAvailableLocationFront`))
  (bind (_fronblockon_x_axis _fronblockon_y_aixs) (break `/Game/Blueprints/Piece_Id` (`self.fronBlockOn`)))
  (bind _currentlyon_x_axis_2 (break `/Game/Blueprints/Piece_Id` (`self.currentlyOn`)))
  ;[1 1 1] find available locations from current location to forward end
  (set `self.fronBlockOn` (make `/Game/Blueprints/Piece_Id` _currentlyon_x_axis_2 9))
  (bind _outactors (`GameplayStatics.GetAllActorsOfClass` "/Game/Blueprints/board_Piece.board_Piece_C"))
  (for _array_element _outactors
    (bind (_id_x_axis _id_y_aixs _id_level) (break `/Game/Blueprints/Piece_Id` (`/Game/Blueprints/board_Piece.id` _array_element)))
    (bind _returnvalue (== (`KismetStringLibrary.GetCharacterAsNumber` _id_x_axis) (`KismetStringLibrary.GetCharacterAsNumber` _currentlyon_x_axis)))
    (bind _returnvalue_2 (> _id_y_aixs _currentlyon_y_aixs))
    (if (and _returnvalue _returnvalue_2 (!= (`/Game/Blueprints/board_Piece.containsColor` _array_element) (`self.color`)))
      (`KismetArrayLibrary.Array_Set` _newavailablelocationfront (`KismetArrayLibrary.Array_Length` _newavailablelocationfront) (make `/Game/Blueprints/Piece_Id` _id_x_axis _id_y_aixs _id_level) true))
    (if (and (`/Game/Blueprints/board_Piece.contains` _array_element) _returnvalue_2 _returnvalue (!= _currentlyon_y_aixs _id_y_aixs))
      (if (> _fronblockon_y_aixs _id_y_aixs)
        (set `self.fronBlockOn` (make `/Game/Blueprints/Piece_Id` _id_x_axis _id_y_aixs _id_level)))))
  (set `self.copyOfFrontLocs` (`self.newAvailableLocationFront`)))

(event `findSideLocation`
  (bind (_currentlyon_x_axis _currentlyon_y_aixs) (break `/Game/Blueprints/Piece_Id` (`self.currentlyOn`)))
  (bind _newavailablelocationleft (`self.newAvailableLocationLeft`))
  (bind _leftblockon_x_axis (break `/Game/Blueprints/Piece_Id` (`self.leftBlockOn`)))
  ;[1 1 1] find all location in left direction, valid and invalid both
  (set `self.leftBlockOn` (make `/Game/Blueprints/Piece_Id` "a"))
  (bind _outactors (`GameplayStatics.GetAllActorsOfClass` "/Game/Blueprints/board_Piece.board_Piece_C"))
  (for _array_element _outactors
    (bind (_id_x_axis _id_y_aixs _id_level) (break `/Game/Blueprints/Piece_Id` (`/Game/Blueprints/board_Piece.id` _array_element)))
    (bind _returnvalue (== _id_y_aixs _currentlyon_y_aixs))
    (bind _returnvalue_2 (`KismetStringLibrary.GetCharacterAsNumber` _id_x_axis))
    (bind _returnvalue_3 (< _returnvalue_2 (`KismetStringLibrary.GetCharacterAsNumber` _currentlyon_x_axis)))
    (if (and _returnvalue _returnvalue_3 (!= (`/Game/Blueprints/board_Piece.containsColor` _array_element) (`self.color`)))
      (`KismetArrayLibrary.Array_Set` _newavailablelocationleft (`KismetArrayLibrary.Array_Length` _newavailablelocationleft) (make `/Game/Blueprints/Piece_Id` _id_x_axis _id_y_aixs _id_level) true))
    (if (and (`/Game/Blueprints/board_Piece.contains` _array_element) _returnvalue_3 _returnvalue (`KismetStringLibrary.NotEqual_StrStr` _id_x_axis _currentlyon_x_axis))
      (if (> _returnvalue_2 (`KismetStringLibrary.GetCharacterAsNumber` _leftblockon_x_axis))
        (set `self.leftBlockOn` (make `/Game/Blueprints/Piece_Id` _id_x_axis _id_y_aixs _id_level)))))
  (set `self.copyOfLeftLocs` (`self.newAvailableLocationLeft`)))

(event `findRIghtLocation`
  (bind (_currentlyon_x_axis _currentlyon_y_aixs) (break `/Game/Blueprints/Piece_Id` (`self.currentlyOn`)))
  (bind _newavailablelocationright (`self.newAvailableLocationRight`))
  (bind _rightblockon_x_axis (break `/Game/Blueprints/Piece_Id` (`self.rightBlockOn`)))
  ;[1 1 1] find all location in right, invalid and valid both
  (set `self.rightBlockOn` (make `/Game/Blueprints/Piece_Id` "z"))
  (bind _outactors (`GameplayStatics.GetAllActorsOfClass` "/Game/Blueprints/board_Piece.board_Piece_C"))
  (for _array_element _outactors
    (bind (_id_x_axis _id_y_aixs _id_level) (break `/Game/Blueprints/Piece_Id` (`/Game/Blueprints/board_Piece.id` _array_element)))
    (bind _returnvalue (== _id_y_aixs _currentlyon_y_aixs))
    (bind _returnvalue_2 (`KismetStringLibrary.GetCharacterAsNumber` _id_x_axis))
    (bind _returnvalue_3 (> _returnvalue_2 (`KismetStringLibrary.GetCharacterAsNumber` _currentlyon_x_axis)))
    (if (and _returnvalue _returnvalue_3 (!= (`/Game/Blueprints/board_Piece.containsColor` _array_element) (`self.color`)))
      (`KismetArrayLibrary.Array_Set` _newavailablelocationright (`KismetArrayLibrary.Array_Length` _newavailablelocationright) (make `/Game/Blueprints/Piece_Id` _id_x_axis _id_y_aixs _id_level) true))
    (if (and (`/Game/Blueprints/board_Piece.contains` _array_element) _returnvalue_3 _returnvalue (`KismetStringLibrary.NotEqual_StrStr` _id_x_axis _currentlyon_x_axis))
      (if (< _returnvalue_2 (`KismetStringLibrary.GetCharacterAsNumber` _rightblockon_x_axis))
        (set `self.rightBlockOn` (make `/Game/Blueprints/Piece_Id` _id_x_axis _id_y_aixs _id_level)))))
  (set `self.copyOfRightLocs` (`self.newAvailableLocationRight`)))

(event `findBackLocation`
  (bind (_currentlyon_x_axis _currentlyon_y_aixs) (break `/Game/Blueprints/Piece_Id` (`self.currentlyOn`)))
  (bind _newavailablelocationback (`self.newAvailableLocationBack`))
  (bind (_backblockon_x_axis _backblockon_y_aixs) (break `/Game/Blueprints/Piece_Id` (`self.backBlockOn`)))
  (bind _currentlyon_x_axis_2 (break `/Game/Blueprints/Piece_Id` (`self.currentlyOn`)))
  ;[1 1 1] find location behind rook, valid and invalid both
  (set `self.backBlockOn` (make `/Game/Blueprints/Piece_Id` _currentlyon_x_axis_2))
  (bind _outactors (`GameplayStatics.GetAllActorsOfClass` "/Game/Blueprints/board_Piece.board_Piece_C"))
  (for _array_element _outactors
    (bind (_id_x_axis _id_y_aixs _id_level) (break `/Game/Blueprints/Piece_Id` (`/Game/Blueprints/board_Piece.id` _array_element)))
    (bind _returnvalue (== (`KismetStringLibrary.GetCharacterAsNumber` _id_x_axis) (`KismetStringLibrary.GetCharacterAsNumber` _currentlyon_x_axis)))
    (bind _returnvalue_2 (> _currentlyon_y_aixs _id_y_aixs))
    (if (and _returnvalue _returnvalue_2 (!= (`/Game/Blueprints/board_Piece.containsColor` _array_element) (`self.color`)))
      (`KismetArrayLibrary.Array_Set` _newavailablelocationback (`KismetArrayLibrary.Array_Length` _newavailablelocationback) (make `/Game/Blueprints/Piece_Id` _id_x_axis _id_y_aixs _id_level) true))
    (if (and (`/Game/Blueprints/board_Piece.contains` _array_element) _returnvalue_2 _returnvalue (!= _currentlyon_y_aixs _id_y_aixs))
      (if (> _id_y_aixs _backblockon_y_aixs)
        (set `self.backBlockOn` (make `/Game/Blueprints/Piece_Id` _id_x_axis _id_y_aixs _id_level)))))
  (set `self.copyOfBackLocs` (`self.newAvailableLocationBack`)))

(fn `UserConstructionScript`)