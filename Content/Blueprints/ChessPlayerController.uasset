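; Player controller for a chess game that toggles the in-game options menu from the Exit Options input action.
; The toggle works only once the ChessGameMode, found with GetAllActorsOfClass, reports that the game has started.
; A visibility flag decides whether to create a new GameOptions widget or to close it with RemoveAllWidgets, which clears every widget rather than just the menu.
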(event `self.ReceiveBeginPlay`)

(event `InputAction|Exit Options`
  (params (Key :type "Key Structure" :default "AnyKey"))
  (:`Pressed`
    (bind _outactors (`GameplayStatics.GetAllActorsOfClass` "/Game/Blueprints/ChessGameMode.ChessGameMode_C"))
    (if (`/Game/Blueprints/ChessGameMode.gameStarted` (`KismetArrayLibrary.Array_Get` _outactors))
      (if (`self.gameOptionsVisible`)
        (`WidgetLayoutLibrary.RemoveAllWidgets`)
        (set `self.gameOptionsVisible` false)
        (else
          (bind _returnvalue (`|CreateWidget` "/Game/Blueprints/GameOptions.GameOptions_C"))
          (`UserWidget.AddToViewport` _returnvalue 0)
          (set `self.gameOptionsVisible` true))))))

(fn `UserConstructionScript`)