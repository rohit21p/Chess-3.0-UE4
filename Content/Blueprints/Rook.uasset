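; Rook chess piece actor that sets its color material and, when clicked, toggles selection through ChessGameMode and highlights the squares it can move to.
; Forward squares are scanned rank by rank until blocked.
; Left, right and back searches collect candidates, track the nearest occupied square and prune anything beyond it, skipping same-color squares.
; Results activate matching Board_Piece actors, and moveTo teleports the rook and deselects it.
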(event `self.ReceiveBeginPlay`
  ;[1 1 1] do this for every rook
  (`self.setMaterial`)
  (`self.setOnClickEvent`)
  (bind _outactors (`GameplayStatics.GetAllActorsOfClass` "/Game/Blueprints/ChessGameMode.ChessGameMode_C"))
  (set `self.gameMode` (`KismetArrayLibrary.Array_Get` _outactors)))

(event `setMaterial`
  ;[1 1 1] set Color
  (if (== (`self.Color`) 1)
    (`PrimitiveComponent.SetMaterial` (`self.Rook`) 0 "/Game/Assets/White_Piece.White_Piece")
    (else
      (`PrimitiveComponent.SetMaterial` (`self.Rook`) 0 "/Game/Assets/Black_Piece.Black_Piece"))))

(event `setOnClickEvent`
  ;[1 1 1] Set what to do on click
  (add `self.OnClicked` (delegate `do`)))

(event `do` :!signature `self.OnClicked`
  (params (TouchedActor :type "Actor Object Reference") (ButtonPressed :type "Key Structure" :default "AnyKey"))
  ;[1 1 1] Set what to do on click
  (`self.onClick`))

(event `onClick`
  ;[1 1 1] on click
  (if (`self.active`)
    (set `self.active` false)
    (`self.setMaterial`)
    (`/Game/Blueprints/ChessGameMode.deactivatePieces` (`self.gameMode`))
    (`KismetArrayLibrary.Array_Clear` (`self.newAvailableLocation`))
    (`KismetArrayLibrary.Array_Clear` (`self.newAvailableLocationRight`))
    (`KismetArrayLibrary.Array_Clear` (`self.newAvailableLocationLeft`))
    (`KismetArrayLibrary.Array_Clear` (`self.newAvailableLocationBack`))
    (else
      (`PrimitiveComponent.SetMaterial` (`self.Rook`) 0 "/Game/Assets/Active_Piece.Active_Piece")
      (`/Game/Blueprints/ChessGameMode.undoSelectOther` (`self.gameMode`))
      (set `self.active` true)
      (set `/Game/Blueprints/ChessGameMode.whoisactive` (`self.id`) (`self.gameMode`))
      (`self.setAvailableLocation`)
      (`self.makeAvailableLocationActive`))))

(event `moveTo`
  (params (Location :type "Vector Structure"))
  ;[1 1 1] move rook to new piece
  (`self.K2_SetActorLocation` Location)
  (`self.onClick`)
  (`KismetArrayLibrary.Array_Clear` (`self.newAvailableLocation`))
  (`KismetArrayLibrary.Array_Clear` (`self.newAvailableLocationRight`))
  (`KismetArrayLibrary.Array_Clear` (`self.newAvailableLocationLeft`))
  (`KismetArrayLibrary.Array_Clear` (`self.newAvailableLocationBack`)))

(event `makeAvailableLocationActive`
  ;[1 1 1] make all available location active
  (for _array_element (`self.NewAvailableLocation`)
    (bind _outactors (`GameplayStatics.GetAllActorsOfClass` "/Game/Blueprints/board_Piece.board_Piece_C"))
    (for _array_element_2 _outactors
      (bind (_id_x_axis _id_y_aixs _id_level) (break `/Game/Blueprints/Piece_Id` (`/Game/Blueprints/board_Piece.id` _array_element_2)))
      (if (and (`KismetStringLibrary.EqualEqual_StrStr` _id_x_axis (break `/Game/Blueprints/Piece_Id` _array_element)) (== _id_y_aixs (`.y_aixs_5_4E9AD4B24CBA9D68C22F87B4D3EBCB46` (break `/Game/Blueprints/Piece_Id` _array_element))) (== _id_level (`.level_9_6EB51A4E4C07ABE6DACD079305A4CC98` (break `/Game/Blueprints/Piece_Id` _array_element))))
        (`PrimitiveComponent.SetMaterial` (`/Game/Blueprints/board_Piece.Piece` _array_element_2) 0 "/Game/Assets/Active_Piece.Active_Piece")
        (set `/Game/Blueprints/board_Piece.active` true _array_element_2)))))

(event `setAvailableLocation`
  ;[1 1 1] find locations, available to move
  (`self.findFrontLocation`)
  (`self.findSideLocation`)
  (`self.findRIghtLocation`)
  (`self.findBackLocation`))

(event `findFrontLocation`
  (bind _newavailablelocation (`self.newAvailableLocation`))
  (bind (_currentlyon_x_axis _currentlyon_y_aixs) (break `/Game/Blueprints/Piece_Id` (`self.currentlyOn`)))
  ;[1 1 1] find available locations from current location to forward end
  (for _index (range (+ _currentlyon_y_aixs 1) 10) :!label _label
    (bind _outactors (`GameplayStatics.GetAllActorsOfClass` "/Game/Blueprints/board_Piece.board_Piece_C"))
    (for _array_element _outactors
      (bind (_id_x_axis _id_y_aixs _id_level) (break `/Game/Blueprints/Piece_Id` (`/Game/Blueprints/board_Piece.id` _array_element)))
      (bind _returnvalue (`KismetStringLibrary.EqualEqual_StrStr` _currentlyon_x_axis _id_x_axis))
      (bind _returnvalue_2 (== _id_y_aixs _index))
      (if (and _returnvalue _returnvalue_2 (!= (`/Game/Blueprints/board_Piece.containsColor` _array_element) (`self.color`)))
        (`KismetArrayLibrary.Array_Set` _newavailablelocation (`KismetArrayLibrary.Array_Length` _newavailablelocation) (make `/Game/Blueprints/Piece_Id` _id_x_axis _id_y_aixs _id_level) true))
      (if (and (`/Game/Blueprints/board_Piece.contains` _array_element) _returnvalue_2 _returnvalue)
        (goto _label :!via `Break`)))))

(event `findSideLocation`
  (bind (_currentlyon_x_axis _currentlyon_y_aixs) (break `/Game/Blueprints/Piece_Id` (`self.currentlyOn`)))
  (bind _newavailablelocationleft (`self.newAvailableLocationLeft`))
  (bind _leftblockon_x_axis (break `/Game/Blueprints/Piece_Id` (`self.leftBlockOn`)))
  (bind _newavailablelocation (`self.newAvailableLocation`))
  ;[1 1 1] find all location in left direction, valid and invalid both
  (set `self.leftBlockOn` (make `/Game/Blueprints/Piece_Id` "a"))
  (bind _outactors (`GameplayStatics.GetAllActorsOfClass` "/Game/Blueprints/board_Piece.board_Piece_C"))
  (for _array_element _outactors
    (bind (_id_x_axis _id_y_aixs _id_level) (break `/Game/Blueprints/Piece_Id` (`/Game/Blueprints/board_Piece.id` _array_element)))
    (bind _returnvalue (== _id_y_aixs _currentlyon_y_aixs))
    (bind _returnvalue_2 (`KismetStringLibrary.GetCharacterAsNumber` _id_x_axis))
    (bind _returnvalue_3 (< _returnvalue_2 (`KismetStringLibrary.GetCharacterAsNumber` _currentlyon_x_axis)))
    (if (and _returnvalue _returnvalue_3 (!= (`/Game/Blueprints/board_Piece.containsColor` _array_element) (`self.color`)))
      (`KismetArrayLibrary.Array_Set` _newavailablelocationleft (`KismetArrayLibrary.Array_Length` _newavailablelocationleft) (make `/Game/Blueprints/Piece_Id` _id_x_axis _id_y_aixs _id_level) true))
    (if (and (`/Game/Blueprints/board_Piece.contains` _array_element) _returnvalue_3 _returnvalue (`KismetStringLibrary.NotEqual_StrStr` _id_x_axis _currentlyon_x_axis))
      (if (> _returnvalue_2 (`KismetStringLibrary.GetCharacterAsNumber` _leftblockon_x_axis))
        (set `self.leftBlockOn` (make `/Game/Blueprints/Piece_Id` _id_x_axis _id_y_aixs _id_level)))))
  (`self.removeBlockedPlaces`)
  (for _array_element_2 (`self.newAvailableLocationLeft`)
    (`KismetArrayLibrary.Array_Set` _newavailablelocation (`KismetArrayLibrary.Array_Length` _newavailablelocation) _array_element_2 true)))

(event `removeBlockedPlaces`
  (bind _leftblockon_x_axis (break `/Game/Blueprints/Piece_Id` (`self.leftBlockOn`)))
  (bind (_backblockon_x_axis _backblockon_y_aixs) (break `/Game/Blueprints/Piece_Id` (`self.backBlockOn`)))
  (bind _rightblockon_x_axis (break `/Game/Blueprints/Piece_Id` (`self.rightBlockOn`)))
  ;[1 1 1] remove invalid locations from left right and back locations
  (for _ (`self.newAvailableLocationLeft`)
    (for _array_element (`self.newAvailableLocationLeft`)
      (if (< (`KismetStringLibrary.GetCharacterAsNumber` (break `/Game/Blueprints/Piece_Id` _array_element)) (`KismetStringLibrary.GetCharacterAsNumber` _leftblockon_x_axis))
        (`KismetArrayLibrary.Array_RemoveItem` (`self.newAvailableLocationLeft`) (make `/Game/Blueprints/Piece_Id` (break `/Game/Blueprints/Piece_Id` _array_element) (`.y_aixs_5_4E9AD4B24CBA9D68C22F87B4D3EBCB46` (break `/Game/Blueprints/Piece_Id` _array_element)) (`.level_9_6EB51A4E4C07ABE6DACD079305A4CC98` (break `/Game/Blueprints/Piece_Id` _array_element)))))))
  (for _ (`self.newAvailableLocationRight`)
    (for _array_element_2 (`self.newAvailableLocationRight`)
      (if (> (`KismetStringLibrary.GetCharacterAsNumber` (break `/Game/Blueprints/Piece_Id` _array_element_2)) (`KismetStringLibrary.GetCharacterAsNumber` _rightblockon_x_axis))
        (`KismetArrayLibrary.Array_RemoveItem` (`self.newAvailableLocationRight`) (make `/Game/Blueprints/Piece_Id` (break `/Game/Blueprints/Piece_Id` _array_element_2) (`.y_aixs_5_4E9AD4B24CBA9D68C22F87B4D3EBCB46` (break `/Game/Blueprints/Piece_Id` _array_element_2)) (`.level_9_6EB51A4E4C07ABE6DACD079305A4CC98` (break `/Game/Blueprints/Piece_Id` _array_element_2)))))))
  (for _ (`self.newAvailableLocationBack`)
    (for _array_element_3 (`self.newAvailableLocationBack`)
      (if (< (`.y_aixs_5_4E9AD4B24CBA9D68C22F87B4D3EBCB46` (break `/Game/Blueprints/Piece_Id` _array_element_3)) _backblockon_y_aixs)
        (`KismetArrayLibrary.Array_RemoveItem` (`self.newAvailableLocationBack`) (make `/Game/Blueprints/Piece_Id` (break `/Game/Blueprints/Piece_Id` _array_element_3) (`.y_aixs_5_4E9AD4B24CBA9D68C22F87B4D3EBCB46` (break `/Game/Blueprints/Piece_Id` _array_element_3)) (`.level_9_6EB51A4E4C07ABE6DACD079305A4CC98` (break `/Game/Blueprints/Piece_Id` _array_element_3))))))))

(event `findRIghtLocation`
  (bind (_currentlyon_x_axis _currentlyon_y_aixs) (break `/Game/Blueprints/Piece_Id` (`self.currentlyOn`)))
  (bind _newavailablelocationright (`self.newAvailableLocationRight`))
  (bind _rightblockon_x_axis (break `/Game/Blueprints/Piece_Id` (`self.rightBlockOn`)))
  (bind _newavailablelocation (`self.newAvailableLocation`))
  ;[1 1 1] find all location in right, invalid and valid both
  (set `self.rightBlockOn` (make `/Game/Blueprints/Piece_Id` "z"))
  (bind _outactors (`GameplayStatics.GetAllActorsOfClass` "/Game/Blueprints/board_Piece.board_Piece_C"))
  (for _array_element _outactors
    (bind (_id_x_axis _id_y_aixs _id_level) (break `/Game/Blueprints/Piece_Id` (`/Game/Blueprints/board_Piece.id` _array_element)))
    (bind _returnvalue (== _id_y_aixs _currentlyon_y_aixs))
    (bind _returnvalue_2 (`KismetStringLibrary.GetCharacterAsNumber` _id_x_axis))
    (bind _returnvalue_3 (> _returnvalue_2 (`KismetStringLibrary.GetCharacterAsNumber` _currentlyon_x_axis)))
    (if (and _returnvalue _returnvalue_3 (!= (`/Game/Blueprints/board_Piece.containsColor` _array_element) (`self.color`)))
      (`KismetArrayLibrary.Array_Set` _newavailablelocationright (`KismetArrayLibrary.Array_Length` _newavailablelocationright) (make `/Game/Blueprints/Piece_Id` _id_x_axis _id_y_aixs _id_level) true))
    (if (and (`/Game/Blueprints/board_Piece.contains` _array_element) _returnvalue_3 _returnvalue (`KismetStringLibrary.NotEqual_StrStr` _id_x_axis _currentlyon_x_axis))
      (if (< _returnvalue_2 (`KismetStringLibrary.GetCharacterAsNumber` _rightblockon_x_axis))
        (set `self.rightBlockOn` (make `/Game/Blueprints/Piece_Id` _id_x_axis _id_y_aixs _id_level)))))
  (`self.removeBlockedPlaces`)
  (for _array_element_2 (`self.newAvailableLocationRight`)
    (`KismetArrayLibrary.Array_Set` _newavailablelocation (`KismetArrayLibrary.Array_Length` _newavailablelocation) _array_element_2 true)))

(event `findBackLocation`
  (bind (_currentlyon_x_axis _currentlyon_y_aixs) (break `/Game/Blueprints/Piece_Id` (`self.currentlyOn`)))
  (bind _newavailablelocationback (`self.newAvailableLocationBack`))
  (bind (_backblockon_x_axis _backblockon_y_aixs) (break `/Game/Blueprints/Piece_Id` (`self.backBlockOn`)))
  (bind _newavailablelocation (`self.newAvailableLocation`))
  (bind _currentlyon_x_axis_2 (break `/Game/Blueprints/Piece_Id` (`self.currentlyOn`)))
  ;[1 1 1] find location behind rook, valid and invalid both
  (set `self.backBlockOn` (make `/Game/Blueprints/Piece_Id` _currentlyon_x_axis_2))
  (bind _outactors (`GameplayStatics.GetAllActorsOfClass` "/Game/Blueprints/board_Piece.board_Piece_C"))
  (for _array_element _outactors
    (bind (_id_x_axis _id_y_aixs _id_level) (break `/Game/Blueprints/Piece_Id` (`/Game/Blueprints/board_Piece.id` _array_element)))
    (bind _returnvalue (== (`KismetStringLibrary.GetCharacterAsNumber` _id_x_axis) (`KismetStringLibrary.GetCharacterAsNumber` _currentlyon_x_axis)))
    (bind _returnvalue_2 (> _currentlyon_y_aixs _id_y_aixs))
    (if (and _returnvalue _returnvalue_2 (!= (`/Game/Blueprints/board_Piece.containsColor` _array_element) (`self.color`)))
      (`KismetArrayLibrary.Array_Set` _newavailablelocationback (`KismetArrayLibrary.Array_Length` _newavailablelocationback) (make `/Game/Blueprints/Piece_Id` _id_x_axis _id_y_aixs _id_level) true))
    (if (and (`/Game/Blueprints/board_Piece.contains` _array_element) _returnvalue_2 _returnvalue (!= _currentlyon_y_aixs _id_y_aixs))
      (if (> _id_y_aixs _backblockon_y_aixs)
        (set `self.backBlockOn` (make `/Game/Blueprints/Piece_Id` _id_x_axis _id_y_aixs _id_level)))))
  (`self.removeBlockedPlaces`)
  (for _array_element_2 (`self.newAvailableLocationBack`)
    (`KismetArrayLibrary.Array_Set` _newavailablelocation (`KismetArrayLibrary.Array_Length` _newavailablelocation) _array_element_2 true)))

(fn `UserConstructionScript`)