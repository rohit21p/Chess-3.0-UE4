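; Bishop chess piece actor that takes a white or black material from its Color value and can be selected by clicking.
; Clicking toggles selection: selecting applies the active material, has ChessGameMode deselect other pieces and records this Id as active, while clicking again restores the color material.
; The game mode is reached through GetAllActorsOfClass.
; MoveTo teleports the bishop to a given location without validation, then runs the click toggle.
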(event `self.ReceiveBeginPlay`
  (`self.setmaterial`)
  (`self.setOnClickEvent`))

(event `setMaterial`
  ;[1 1 1] set Color
  (if (== (`self.Color`) 1)
    (`PrimitiveComponent.SetMaterial` (`self.Bishop`) 0 "/Game/Assets/White_Piece.White_Piece")
    (else
      (`PrimitiveComponent.SetMaterial` (`self.Bishop`) 0 "/Game/Assets/Black_Piece.Black_Piece"))))

(event `setOnClickEvent`
  ;[1 1 1] Set what to do on click
  (add `self.OnClicked` (delegate `do`)))

(event `do` :!signature `self.OnClicked`
  (params (TouchedActor :type "Actor Object Reference") (ButtonPressed :type "Key Structure" :default "AnyKey"))
  ;[1 1 1] Set what to do on click
  (`self.onClick`))

(event `onClick`
  ;[1 1 1] on click
  (if (`self.active`)
    (set `self.active` false)
    (`self.setMaterial`)
    (else
      (`PrimitiveComponent.SetMaterial` (`self.Bishop`) 0 "/Game/Assets/Active_Piece.Active_Piece")
      (bind _outactors (`GameplayStatics.GetAllActorsOfClass` "/Game/Blueprints/ChessGameMode.ChessGameMode_C"))
      (for _array_element _outactors
        (`/Game/Blueprints/ChessGameMode.undoSelectOther` _array_element)
        (set `self.active` true)
        (set `/Game/Blueprints/ChessGameMode.whoisactive` (`self.id`) _array_element)))))

(event `moveTo`
  (params (Location :type "Vector Structure"))
  ;[1 1 1] move bishop to new piece
  (`self.K2_SetActorLocation` Location)
  (`self.onClick`))

(fn `UserConstructionScript`)